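; BP_Medaillon is the Witcher player's medallion, meant to detect nearby enemies and magic.
; Its collision sphere's begin-overlap event passes the other actor to ReactEnemyOrMagic, which casts it to BP_Enemy and checks the enemy tag.
; The reaction is only a debug string print for a found or missing tag.
; A matching BP_MagicCube tag check exists but is disconnected, so magic detection never runs.
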(event `self.MedailonSphereCollisionComponent.OnComponentBeginOverlap`
  (params (OverlappedComponent :type "PrimitiveComponent Object Reference") (OtherActor :type "Actor Object Reference") (OtherComp :type "PrimitiveComponent Object Reference") (OtherBodyIndex :type Integer) (bFromSweep :type Boolean) (SweepResult :type "HitResult Structure (by ref)"))
  ;[1 1 1] FCS For detecting enemy and magic
  (`self.ReactEnemyOrMagic` OtherActor OtherActor))

(fn `ReactEnemyOrMagic`
  (params (Object :type "Object Object Reference") (Object2 :type "Object Object Reference"))
  (bind _enemytag (`self.EnemyTag`))
  (bind _asbp_enemy (cast `/Game/TheWitcher/Enemy/BP_Enemy` Object))
  (if (`self.ActorHasTag` _asbp_enemy _enemytag)
    (`KismetSystemLibrary.PrintString` (`KismetStringLibrary.Concat_StrStr` "BP_Medailon" " OVERALAPUJE S " (`KismetStringLibrary.Conv_NameToString` _enemytag)))
    (else
      (`KismetSystemLibrary.PrintString` "Nebyl nalezen žádný tag pro enemy"))))

(fn `UserConstructionScript`)